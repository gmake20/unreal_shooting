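; BP_Enemy is an enemy that flies in a straight line toward the player's starting position and explodes on overlap.
; BeginPlay finds BP_Player and FindDirection sets a one-time heading, aligning local Z to it.
; The random roll always passes, so straight down applies only without a valid player.
; Tick moves it without sweep; Box overlap spawns explosion effects and destroys both actors.
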(event `self.ReceiveBeginPlay`
  (bind _returnvalue (`GameplayStatics.GetActorOfClass` "/Game/Blueprints/BP_Player.BP_Player_C"))
  (bind _output_get (set `self.Target` _returnvalue))
  (`self.FindDirection` _output_get))

(event `self.ReceiveTick`
  (params (DeltaSeconds :type "Float (single-precision)"))
  ;[1 1 1] 이동하고싶다.
  ;;[1 1 1] P
  (`self.K2_SetActorLocation` (+ (* DeltaSeconds (* (`self.Direction`) (`self.Speed`))) (`self.K2_GetActorLocation`))))

(event `self.Box.OnComponentBeginOverlap`
  (params (OverlappedComponent :type "PrimitiveComponent Object Reference") (OtherActor :type "Actor Object Reference") (OtherComp :type "PrimitiveComponent Object Reference") (OtherBodyIndex :type Integer) (bFromSweep :type Boolean) (SweepResult :type "HitResult Structure (by ref)"))
  ;[1 1 1] 충돌하면 충돌체도 파괴되고 나도 파괴된다.
  (`GameplayStatics.SpawnEmitterAtLocation` "/Game/StarterContent/Particles/P_Explosion.P_Explosion" (`self.K2_GetActorLocation`))
  (`GameplayStatics.PlaySound2D` "/Game/Sound/Explosion.Explosion" 1.0 1.0 0.0 null null)
  (`self.K2_DestroyActor` OtherActor)
  (`self.K2_DestroyActor`))

(fn `FindDirection`
  (params (InputObject :type "Object Object Reference"))
  ;[1 1 1] 방향을 구한다.
  (`/Engine/EditorBlueprintResources/StandardMacros.IsValid` InputObject
    (:`Is Valid`
      (if (<= (`KismetMathLibrary.RandomIntegerInRange` 1 10) 10)
        (set `self.Direction` (`KismetMathLibrary.Normal` (- (`self.K2_GetActorLocation` (`self.Target`)) (`self.K2_GetActorLocation`))))
        (else
          (set `self.Direction` (0.0 0.0 -1.0) :!label _label))))
    (:`Is Not Valid`
      (goto _label)))
  (`self.K2_SetActorRotation` (`KismetMathLibrary.MakeRotFromXZ` (`self.GetActorForwardVector`) (`self.Direction`))))

(fn `UserConstructionScript`)