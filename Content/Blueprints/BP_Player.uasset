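; BP_Player is the player-controlled actor that moves in the Y-Z plane and shoots bullets.
; Horizontal and Vertical axis events share one setter for Direction, which Tick scales by Speed and delta time for a swept location update.
; Pressing Fire spawns BP_Bullet at the FirePosition component and plays a blaster sound.
; A Plus helper function adds two numbers but is not called in these graphs.
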(event `self.ReceiveBeginPlay`)

(event `self.ReceiveTick`
  (params (DeltaSeconds :type "Float (single-precision)"))
  ;[1 1 1] 이동하고싶다.
  ;;[1 1 1] P
  (`self.K2_SetActorLocation` (+ (* DeltaSeconds (* (`self.Direction`) (`self.Speed`))) (`self.K2_GetActorLocation`)) true))

(event `InputAxis|Horizontal`
  (params (AxisValue :type "Float (single-precision)"))
  ;[1 1 1] 방향을 구한다.
  (set `self.Direction` (`KismetMathLibrary.MakeVector` 0.0 AxisValue (stale `InputAxis|Vertical` AxisValue)) :!label _label))

(event `InputAxis|Vertical`
  (params (AxisValue :type "Float (single-precision)"))
  ;[1 1 1] 방향을 구한다.
  (goto _label))

(event `InputAction|Fire`
  (params (Key :type "Key Structure"))
  (:`Pressed`
    (`|SpawnActorFromClass` "/Game/Blueprints/BP_Bullet.BP_Bullet_C" (`KismetMathLibrary.MakeTransform` (`SceneComponent.K2_GetComponentLocation` (`self.FirePosition`))) "Undefined" "MultiplyWithRoot" null null)
    (`GameplayStatics.PlaySound2D` "/Game/Sound/star-wars-blaster.star-wars-blaster" 0.2 1.0 0.0 null null)))

(fn `Plus`
  (params (Number1 :type Integer) (Number2 :type Integer))
  (returns (Result :type Integer))
  (return (+ Number1 Number2)))

(fn `UserConstructionScript`)